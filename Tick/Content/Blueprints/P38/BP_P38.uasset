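; Player-controlled P38 plane pawn that constantly flies forward, steers by pitch and roll axis input, and fires rockets.
; BeginPlay registers both propeller meshes with the BPRotate component for spinning.
; Tick feeds forward movement input and switches FloatingPawnMovement max speed from a boost flag set by holding Speed Up.
; Tick also drives a delay-based flicker of the left and right lights.
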(event Custom|Speed_UP
  ;[1 1 1] Move & Speed Up
  (Variables|Default|SetSpeed_Up_OnOff true))

(event Custom|Speed_UP_Stop
  ;[1 1 1] Move & Speed Up
  (Variables|Default|SetSpeed_Up_OnOff false))

(event Custom|Light_Toggle
  ;[1 1 1] Light Flicker
  (Rendering|ToggleVisibility (Variables|Default|GetLight_R) false))

(event EventBeginPlay
  ;[1 1 1] Rotate
  (Utilities|Array|Add (Variables|/Game/Blueprints/BP_Rotate.BP_Rotate_C|GetScene (Variables|Default|GetBP_Rotate)) (Variables|Default|GetSM_P38_Propeller))
  (Utilities|Array|Add (Variables|/Game/Blueprints/BP_Rotate.BP_Rotate_C|GetScene (Variables|Default|GetBP_Rotate)) (Variables|Default|GetSM_P38_Propeller1)))

(event EventTick
  (params (DeltaSeconds :type Float%20%28single-precision%29))
  (bind _floatingpawnmovement (Variables|Default|GetFloatingPawnMovement))
  ;[1 1 1] Move & Speed Up
  (Utilities|FlowControl|Sequence
    (:then_0
      (Pawn|Input|AddMovementInput (Transformation|GetActorForwardVector) 1.0 false))
    (:then_1
      (if (Variables|Default|GetSpeed_Up_OnOff)
        (Variables|/Script/Engine.FloatingPawnMovement|SetMaxSpeed _floatingpawnmovement 2e+03)
        (else
          (Variables|/Script/Engine.FloatingPawnMovement|SetMaxSpeed _floatingpawnmovement 1e+03))))
    (:then_2
      ;[1 1 1] Light Flicker
      (Utilities|FlowControl|Delay 2.0)
      (CallFunction|LightToggle)
      (Utilities|FlowControl|Delay 5.0)
      (Class|TypedElementListLibrary|Reset))))

(event Input|ActionEvents|InputActionFire
  (params (Key :type Key%20Structure :default "None"))
  ;[1 1 1] Rocket Fire
  (:Pressed
    (Game|SpawnActorfromClass "/Game/Blueprints/Rocket/BP_Rocket.BP_Rocket_C" (Transformation|GetActorTransform) "Undefined" "MultiplyWithRoot" 0 0)))

(event Input|ActionEvents|InputActionSpeedUp
  (params (Key :type Key%20Structure :default "None"))
  ;[1 1 1] Move & Speed Up
  (:Pressed
    (CallFunction|SpeedUP))
  (:Released
    (CallFunction|SpeedUPStop)))

(event Input|AxisEvents|InputAxisPitch
  (params (AxisValue :type Float%20%28single-precision%29))
  ;[1 1 1] Controll
  (Transformation|AddActorLocalRotation (Math|Rotator|MakeRotator 0.0 (* AxisValue (Variables|Default|GetRotateSpeed) (Utilities|Time|GetWorldDeltaSeconds)) 0.0) false false))

(event Input|AxisEvents|InputAxisRoll
  (params (AxisValue :type Float%20%28single-precision%29))
  ;[1 1 1] Controll
  (Transformation|AddActorLocalRotation (Math|Rotator|MakeRotator (* AxisValue (Variables|Default|GetRotateSpeed) (Utilities|Time|GetWorldDeltaSeconds)) 0.0 0.0) false false))

(fn ConstructionScript)